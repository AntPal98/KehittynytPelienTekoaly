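; Behavior tree task that has the friend robot relieve homesickness by visiting its GazingPoint actor.
; It issues a move to that point and immediately sets the robot's rotation from only the Y offset toward it, without waiting for arrival.
; After a short fixed delay, it records the robot's time since creation as PreviousCureTime on the AI controller, then finishes successfully.
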(event `self.ReceiveExecuteAI`
  (params (OwnerController :type "AIController Object Reference") (ControlledPawn :type "Pawn Object Reference"))
  (bind _asfriend_robot_bp (cast `/Game/Blueprints/FriendRobot_BP` ControlledPawn))
  (bind _gazingpoint (`/Game/Blueprints/FriendRobot_BP.GazingPoint` _asfriend_robot_bp))
  (`AIController.MoveToActor` OwnerController _gazingpoint -1.0 true true true null true)
  (`Actor.K2_SetActorRotation` _asfriend_robot_bp (`KismetMathLibrary.Conv_VectorToRotator` (`KismetMathLibrary.MakeVector` 0.0 (.y (- (`Actor.K2_GetActorLocation` _gazingpoint) (`Actor.K2_GetActorLocation` _asfriend_robot_bp))))) false)
  (`KismetSystemLibrary.Delay` 2.0)
  (bind _asfriend_robot_aicontroller (cast `/Game/Blueprints/AI_Blueprints/FriendRobot_AIController` (`Pawn.GetController` (`Actor.Instigator` OwnerController))))
  (set `/Game/Blueprints/AI_Blueprints/FriendRobot_AIController.PreviousCureTime` (`Actor.GetGameTimeSinceCreation` _asfriend_robot_bp) _asfriend_robot_aicontroller)
  (`self.FinishExecute` true))