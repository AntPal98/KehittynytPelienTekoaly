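; OviSparks is an actor that pairs an animated skeletal mesh with a particle system, showing sparks while the mesh animates.
; The Sparks emitter starts disabled, and Tick sets its enabled state to match whether the mesh is playing.
; A looping two-second timer randomizes the animation's play rate within a slow range.
; The timer also sends a separate random float to the particle system, but its parameter name is None.
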(event `self.ReceiveBeginPlay`
  (`parent.ReceiveBeginPlay`)
  (`FXSystemComponent.SetEmitterEnable` (`self.ParticleSystem`) "Sparks" false)
  (`KismetSystemLibrary.K2_SetTimer` null "PlayRateChange" 2.0 true))

(event `self.ReceiveTick`
  (params (DeltaSeconds :type "Float (single-precision)"))
  (`parent.ReceiveTick` DeltaSeconds)
  (`FXSystemComponent.SetEmitterEnable` (`self.ParticleSystem`) "Sparks" (`SkeletalMeshComponent.IsPlaying` (`self.SkeletalMeshComponent`))))

(fn `PlayRateChange`
  (bind _returnvalue (`KismetMathLibrary.RandomFloatInRange` 0.1 0.5))
  (`SkeletalMeshComponent.SetPlayRate` (`self.SkeletalMeshComponent`) _returnvalue)
  (`FXSystemComponent.SetFloatParameter` (`self.ParticleSystem`) "None" _returnvalue))

(fn `UserConstructionScript`
  (`parent.UserConstructionScript`))