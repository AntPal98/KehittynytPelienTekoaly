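; BP_TerminalScreen is a terminal screen actor that displays lines of text on its static mesh.
; On BeginPlay it creates a canvas render target and feeds it into a dynamic M_TerminalScreen material on the mesh.
; The render target's update event draws each TerminalText entry as a separate row in the terminal font.
; A one-shot timer later swaps in placeholder strings and calls UpdateResource to redraw the screen.
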(event `self.ReceiveBeginPlay`
  (`|ExecutionSequence`
    (:`then_0`
      (bind _returnvalue (`CanvasRenderTarget2D.CreateCanvasRenderTarget2D` "/Game/Blueprints/Terminal/CRT_Terminal.CRT_Terminal_C"))
      (bind _output_get (set `self.ScreenTest` _returnvalue))
      (add `CanvasRenderTarget2D.OnCanvasRenderTargetUpdate` _output_get (delegate `RenderTextEvent`))
      (`CanvasRenderTarget2D.UpdateResource` (`self.ScreenTest`)))
    (:`then_1`
      (bind _returnvalue_2 (`KismetMaterialLibrary.CreateDynamicMaterialInstance` "/Game/Blueprints/Terminal/M_TerminalScreen.M_TerminalScreen"))
      (`PrimitiveComponent.SetMaterial` (`self.StaticMesh`) 0 _returnvalue_2)
      (`MaterialInstanceDynamic.SetTextureParameterValue` _returnvalue_2 "ScreenTexture" (`self.ScreenTest`)))
    (:`then_2`
      (`KismetSystemLibrary.K2_SetTimerDelegate` (delegate `ChangeText`) 5.0))))

(event `RenderTextEvent`
  (params (Canvas :type "Canvas Object Reference") (Width :type Integer) (Height :type Integer))
  (for (_array_element _array_index) (`self.TerminalText`)
    (`Canvas.K2_DrawText` Canvas "/Game/Blueprints/Terminal/DS-TERM_Font.DS-TERM_Font" _array_element (`KismetMathLibrary.MakeVector2D` 100.0 (* _array_index 100.0)) (2.0 2.0) (struct :`R` 1.0 :`G` 1.0 :`B` 1.0 :`A` 1.0) 0.0 (struct :`A` 1.0) (1.0 1.0) false false false (struct :`A` 1.0))))

(event `ChangeText`
  (set `self.TerminalText` (`|MakeArray` "Adsads" "asdada" "dasdad"))
  (`CanvasRenderTarget2D.UpdateResource` (`self.ScreenTest`)))

(fn `UserConstructionScript`)